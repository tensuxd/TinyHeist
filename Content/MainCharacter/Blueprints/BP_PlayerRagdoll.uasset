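; BP_PlayerRagdoll is a player character Blueprint with sprinting and object-interaction helpers; despite its name, it shows no ragdoll logic.
; Client and server sprint events feed SetSprint, which switches max walk speed between run and sprint.
; InteractTrace line-traces from Target for WorldDynamic and Pawn objects, while CleanObjVariables resets interaction state.
; Much looks unfinished: Fixate's player-freezing branch never runs, and double-jump and InteractPoint nodes are unconnected.
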(event Custom|Sprint%20ON%20Server
  ;[0.15 0.15 0.15 0.5] Replication Sprint
  (CallFunction|SetSprint true))

(event Custom|Sprint%20OFF%20Client
  ;[0.15 0.15 0.15 0.5] Replication Sprint
  (CallFunction|SetSprint false))

(event Custom|Sprint%20ON%20Client
  ;[0.15 0.15 0.15 0.5] Replication Sprint
  (CallFunction|SetSprint true))

(event Custom|Sprint%20OFF%20Server
  ;[0.15 0.15 0.15 0.5] Replication Sprint
  (CallFunction|SetSprint false))

(fn ConstructionScript)

(fn InteractTrace
  (params (Distance :type Integer))
  (bind _target (Variables|Default|Gettarget))
  (bind (_outhit _returnvalue) (Collision|LineTraceForObjects (Transformation|GetWorldLocation _target) (.Output_Loc (Utilities|InteractPoint _target Distance)) (Utilities|Array|MakeArray "ObjectTypeQuery2" "ObjectTypeQuery3") false 0 "ForDuration"))
  (return _returnvalue (.HitActor (Collision|BreakHitResult _outhit)) (.HitComponent (Collision|BreakHitResult _outhit)) (.Location (Collision|BreakHitResult _outhit))))

(fn Fixate
  (params (Comp :type Primitive%20Component%20Object%20Reference) (Actor :type Actor%20Object%20Reference))
  (if (not true)
    (if (not (Physics|IsSimulatingPhysics Comp "None"))
      (bind _asbp_player (Utilities|Casting|CastToBP_Player Actor))
      (Variables|Interact|SetAs%20AnotherPlayer _asbp_player)
      (Pawn|Components|CharacterMovement|DisableMovement (Variables|/Script/Engine.Character|GetCharacterMovement (Variables|Interact|GetAs%20AnotherPlayer)))
      (Development|PrintString "I got a player" true true "(R=0.000000,G=1.000000,B=0.022319,A=1.000000)"))))

(fn SetSprint
  (params (Enable :type Boolean))
  (bind _charactermovement (Variables|Character|GetCharacterMovement))
  (if Enable
    (Variables|Movement|Speed|SetisSprinting? true)
    (Variables|/Script/Engine.CharacterMovementComponent|SetMaxWalkSpeed _charactermovement (Variables|Movement|Speed|GetMax%20Sprint%20Speed))
    (else
      (Variables|Movement|Speed|SetisSprinting? false)
      (Variables|/Script/Engine.CharacterMovementComponent|SetMaxWalkSpeed _charactermovement (Variables|Movement|Speed|GetMax%20Run%20Speed)))))

(fn SetInteractionParameter
  (return true))