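; DoorBP is a level environment door Blueprint with an OpenShelf function that creates a handle actor for manipulating a component.
; When GetRelease is true, OpenShelf spawns a Dir actor, attaches it to the passed component with welding, moves it to the impact point and returns it.
; A physics constraint step linking that component to the Dir sphere is disconnected.
; The interaction parameter function just returns false, and the construction script is empty.
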(fn ConstructionScript)

(fn SetInteractionParameter
  (return false))

(fn OpenShelf
  (params (Get/Release :type Boolean) (Impact%20Point :type Vector :default "0, 0, 0") (NewParam :type Primitive%20Component%20Object%20Reference))
  (if Get/Release
    (bind _returnvalue (Game|SpawnActorfromClass "/Game/Levels/Environment/Dir.Dir_C" (Math|Transform|MakeTransform "0, 0, 0" "0, 0, 0" "1.000000,1.000000,1.000000") "AlwaysSpawn" "MultiplyWithRoot" 0 0))
    (bind _output_get (Variables|Default|SetNewVar _returnvalue))
    (Transformation|AttachComponentToComponent _output_get NewParam "None" "KeepWorld" "KeepWorld" "KeepWorld" true)
    (Transformation|SetActorLocation _output_get Impact%20Point false false)
    (return _output_get)))